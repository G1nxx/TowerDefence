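; MyBasicBullet is a bullet actor that damages enemies when its Sphere component begins overlapping them.
; Actor tags select the BasicEnemy or StrongEnemy branch, which casts to that enemy class, calls its TakeDamage and prints a debug message.
; Damage scales linearly with LevelOfDamage, with strong enemies receiving about 80% of the basic-enemy amount.
; The bullet destroys itself after either tag match and ignores all other overlaps.
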(event OnComponentBeginOverlap(Sphere)
  (params (OverlappedComponent :type Primitive%20Component%20Object%20Reference) (OtherActor :type Actor%20Object%20Reference) (OtherComp :type Primitive%20Component%20Object%20Reference) (OtherBodyIndex :type Integer) (bFromSweep :type Boolean) (SweepResult :type Hit%20Result%20Structure%20%28by%20ref%29))
  (if (Actor|ActorHasTag OtherActor "BasicEnemy")
    (bind _asmy_basic_enemy (Utilities|Casting|CastToMyBasicEnemy OtherActor)
      (:then
        (Class|AbstractEnemy|TakeDamage _asmy_basic_enemy (/ (* (Variables|Default|Getdamage) (+ (Variables|Default|GetlevelOfDamage) 10)) 10))
        (Development|PrintString "BasicEnemyTouched" true true "(R=1.000000,G=0.567016,B=0.151122,A=1.000000)"))
      (:CastFailed
        _))
    (Actor|DestroyActor)
    (elif (Actor|ActorHasTag OtherActor "StrongEnemy")
      (bind _asmy_strong_enemy (Utilities|Casting|CastToMyStrongEnemy OtherActor)
        (:then
          (Class|AbstractEnemy|TakeDamage _asmy_strong_enemy (* (/ (* (Variables|Default|Getdamage) (+ (Variables|Default|GetlevelOfDamage) 10)) 100) 8))
          (Development|PrintString "StrongEnemyTouched" true true "(R=1.000000,G=0.567016,B=0.151122,A=1.000000)"))
        (:CastFailed
          _))
      (Actor|DestroyActor))))

(fn ConstructionScript)