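; MySplashBullet is a splash-damage projectile that damages a group of enemies when it hits one.
; When its Sphere overlaps an actor tagged Enemy, it damages every AbstractEnemy inside DamageSphere, then destroys itself.
; Damage scales with LevelOfDamage, and enemies tagged StrongEnemy take a reduced share.
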(event OnComponentBeginOverlap(Sphere)
  (params (OverlappedComponent :type Primitive%20Component%20Object%20Reference) (OtherActor :type Actor%20Object%20Reference) (OtherComp :type Primitive%20Component%20Object%20Reference) (OtherBodyIndex :type Integer) (bFromSweep :type Boolean) (SweepResult :type Hit%20Result%20Structure%20%28by%20ref%29))
  (bind _damage (Variables|Default|Getdamage))
  (bind _levelofdamage (Variables|Default|GetlevelOfDamage))
  (bind _returnvalue (+ _levelofdamage 10))
  (bind _returnvalue_2 (* _damage _returnvalue))
  (bind _returnvalue_3 (/ _returnvalue_2 10))
  (if (Actor|ActorHasTag OtherActor "Enemy")
    (bind _array_element (Utilities|Array|ForEachLoopwithBreak (Collision|GetOverlappingActors (Variables|Default|GetDamageSphere) "/Script/TowerDefence.AbstractEnemy" :!class /Script/Engine.PrimitiveComponent))
      (:LoopBody
        (bind _asabstract_enemy (Utilities|Casting|CastToAbstractEnemy _array_element))
        (if (Actor|ActorHasTag _asabstract_enemy "StrongEnemy")
          (Class|AbstractEnemy|TakeDamage _asabstract_enemy (* (/ _returnvalue_3 10) 8))
          (else
            (Class|AbstractEnemy|TakeDamage _asabstract_enemy _returnvalue_3))))
      (:Completed
        (Actor|DestroyActor)))))

(fn ConstructionScript)