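; Main base of a tower defense game, holding the player's money and base health and driving the UI.
; BeginPlay sets starting values, then calls UpdateInterface after a brief delay.
; UpdateInterface refreshes health, money and wave text, and enables tower build and upgrade buttons by affordability, finding actors via GetActorOfClass.
; BaseDestroyedEvent repositions the death screen actor's height and pauses the game after a short delay.
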(event Custom|UpdateInterface
  (bind _moneyingame (Variables|Default|GetMoneyInGame))
  (bind _asinterface (Utilities|Casting|CastToInterface (UserInterface|GetWidget (Variables|Default|GetIntrface))))
  (bind _returnvalue (Actor|GetActorOfClass "MyMainBase_C"))
  (Variables|/Script/UMG.TextBlock|SetText (Variables|/Game/Blueprints/UI/Widgets/Interface.Interface_C|GetTextBlock_Health _asinterface) (Utilities|Text|ToText(Integer) (Variables|/Script/TowerDefence.MainBase|GetHealthOfMainBase _returnvalue)))
  (Variables|/Script/UMG.TextBlock|SetText (Variables|/Game/Blueprints/UI/Widgets/Interface.Interface_C|GetTextBlock_Money _asinterface) (Utilities|Text|ToText(Integer) (Variables|/Script/TowerDefence.MainBase|GetMoneyInGame _returnvalue)))
  (bind _returnvalue_2 (Actor|GetActorOfClass "/Game/Blueprints/Components/MySpawnerFirst.MySpawnerFirst_C"))
  (if (> (- (Variables|/Script/TowerDefence.Spawner|GetWaveCount _returnvalue_2) 1) 0)
    (Variables|/Script/UMG.TextBlock|SetText (Variables|/Game/Blueprints/UI/Widgets/Interface.Interface_C|GetTextBlock_WaveCount _asinterface) (Utilities|Text|ToText(Integer) (- (Variables|/Script/TowerDefence.Spawner|GetWaveCount _returnvalue_2) 1)))
    (else
      (Variables|/Script/UMG.TextBlock|SetText (Variables|/Game/Blueprints/UI/Widgets/Interface.Interface_C|GetTextBlock_WaveCount _asinterface) "0")))
  (bind _returnvalue_3 (Actor|GetActorOfClass "/Game/Blueprints/UI/MenuForBuilding.MenuForBuilding_C"))
  (bind _astower_widget (Utilities|Casting|CastToTowerWidget (UserInterface|GetWidget (Variables|/Game/Blueprints/UI/MenuForBuilding.MenuForBuilding_C|GetWidget _returnvalue_3))))
  (Widget|SetIsEnabled (Variables|/Game/Blueprints/UI/Widgets/TowerWidget.TowerWidget_C|GetBasicTowerButton _astower_widget) (>= _moneyingame (Variables|Default|GetBasicTowerCost)))
  (Widget|SetIsEnabled (Variables|/Game/Blueprints/UI/Widgets/TowerWidget.TowerWidget_C|GetSplashTowerButton _astower_widget) (>= _moneyingame (Variables|Default|GetSplashTowerCost)))
  (Widget|SetIsEnabled (Variables|/Game/Blueprints/UI/Widgets/TowerWidget.TowerWidget_C|GetSniperTowerButton _astower_widget) (>= _moneyingame (Variables|Default|GetSniperTowerCost)))
  (bind _returnvalue_4 (Actor|GetActorOfClass "/Game/Blueprints/UI/MenuForUpgrading.MenuForUpgrading_C"))
  (bind _asupgrade_widget (Utilities|Casting|CastToUpgradeWidget (UserInterface|GetWidget (Variables|/Game/Blueprints/UI/MenuForUpgrading.MenuForUpgrading_C|GetWidget _returnvalue_4))))
  (Widget|SetIsEnabled (Variables|/Game/Blueprints/UI/Widgets/UpgradeWidget.UpgradeWidget_C|GetUpgradeButton _asupgrade_widget) (> (Variables|Default|GetMoneyInGame) (Variables|Default|GetMoneyForUpgrade))))

(event EventBeginPlay
  (Variables|Default|SetMoneyInGame 200)
  (Variables|Default|SetHealthOfMainBase 20)
  (Utilities|FlowControl|Delay 0.01)
  (CallFunction|UpdateInterface))

(event EventTick
  (params (DeltaSeconds :type Float%20%28single-precision%29)))

(event EventBaseDestroyedEvent
  (bind _returnvalue (Actor|GetActorOfClass "/Game/Blueprints/UI/DeathScreen_BP1.DeathScreen_BP1_C"))
  (Transformation|SetActorLocation _returnvalue (Math|Vector|MakeVector (.x (Transformation|GetActorLocation _returnvalue)) (.y (Transformation|GetActorLocation _returnvalue)) 2e+02) false false)
  (Utilities|FlowControl|Delay 0.02)
  (Game|SetGamePaused true))

(fn ConstructionScript)