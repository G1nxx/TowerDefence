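; Enemy spawner Blueprint that configures enemy waves and triggers the win screen after the final one.
; BeginPlay sets the enemy count, class and spawn timer, and Tick re-randomises that timer every frame; no spawning logic is in this graph.
; NewWave refreshes the main base's interface.
; FinalWave polls through a short Delay loop until no AbstractEnemy remains, then repositions the WinScreen actor vertically and pauses the game.
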(event EventBeginPlay
  (Variables|Default|SetEnemiesCount 10)
  (Variables|Default|SetEnemyActor "/Game/Blueprints/Enemies/MyBasicEnemy.MyBasicEnemy_C")
  (Variables|Default|SetSpawnTimer 0.3))

(event EventNewWave
  (bind _returnvalue (Actor|GetActorOfClass "/Game/Blueprints/Components/MyMainBase.MyMainBase_C"))
  (Default|UpdateInterface _returnvalue))

(event EventTick
  (params (DeltaSeconds :type Float%20%28single-precision%29))
  (Variables|Default|SetSpawnTimer (Math|Random|RandomFloatinRange 0.2 0.4)))

(event EventFinalWave
  (bind _outactors (Actor|GetAllActorsOfClass "/Script/TowerDefence.AbstractEnemy" :!label _label))
  (if (<= (Utilities|Array|Length _outactors) 0)
    (bind _returnvalue (Actor|GetActorOfClass "/Game/Blueprints/UI/WinScreen_BP1.WinScreen_BP1_C"))
    (Transformation|SetActorLocation _returnvalue (Math|Vector|MakeVector (.x (Transformation|GetActorLocation _returnvalue)) (.y (Transformation|GetActorLocation _returnvalue)) 2e+02) false false)
    (Utilities|FlowControl|Delay 0.02)
    (Game|SetGamePaused true)
    (else
      (Utilities|FlowControl|Delay 0.01)
      (goto _label))))

(fn ConstructionScript)