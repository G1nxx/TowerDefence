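; PlaceToBuild is an actor marking a tower build spot, with a Paper2D sprite that starts hidden.
; The sprite's click event finds the MenuForBuilding actor, registers this spot as its tower place to interact and shows the menu widget.
; It then hides the sprites of all PlaceToBuild actors and reveals its own, so only the selected spot is visible.
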(event OnClicked(PaperSprite)
  (params (TouchedComponent :type Primitive%20Component%20Object%20Reference) (ButtonPressed :type Key%20Structure))
  (Development|PrintString "Hello")
  (bind _returnvalue (Actor|GetActorOfClass "/Game/Blueprints/UI/MenuForBuilding.MenuForBuilding_C"))
  (Variables|/Game/Blueprints/UI/MenuForBuilding.MenuForBuilding_C|SetTowerPlaceToInteract _returnvalue self)
  (Default|ShowWidget _returnvalue)
  (bind _outactors (Actor|GetAllActorsOfClass "PlaceToBuild_C"))
  (for _array_element _outactors
    (Rendering|SetVisibility (Variables|PlaceToBuild_C|GetPaperSprite _array_element) false false))
  (Rendering|SetVisibility (Variables|Default|GetPaperSprite) true false))

(event EventBeginPlay
  (Rendering|SetVisibility (Variables|Default|GetPaperSprite) false false))

(fn ConstructionScript)