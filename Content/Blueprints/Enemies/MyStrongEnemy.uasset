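; Strong enemy Blueprint that damages the main base on reaching it and pays out money when killed.
; BeginPlay sets its kill reward, while the base-reached and killed events each look up MyMainBase by class to adjust its health or money directly.
; Both events refresh the base's interface, print a debug string and then share a single destroy step.
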(event EventEnemyIsKilled
  ;[1 1 1] EnemyIsKilled
  (bind _returnvalue (Actor|GetActorOfClass "/Game/Blueprints/Components/MyMainBase.MyMainBase_C"))
  (bind _output_get (Variables|/Script/TowerDefence.MainBase|SetMoneyInGame _returnvalue (Math|Float|Truncate (+ (Variables|/Script/TowerDefence.MainBase|GetMoneyInGame _returnvalue) (Variables|Default|GetValueForKilling)))))
  (Default|UpdateInterface _returnvalue)
  (Development|PrintString (Utilities|String|ToString(Integer) _output_get) true true "(R=0.040479,G=1.000000,B=0.074658,A=1.000000)")
  (Actor|DestroyActor))

(event EventBeginPlay
  (Variables|Default|SetValueForKilling 3))

(event EventEnemyatBase
  ;[1 1 1] EnemyAtBase
  (bind _returnvalue (Actor|GetActorOfClass "/Game/Blueprints/Components/MyMainBase.MyMainBase_C"))
  (Variables|/Script/TowerDefence.MainBase|SetHealthOfMainBase _returnvalue (- (Variables|/Script/TowerDefence.MainBase|GetHealthOfMainBase _returnvalue) 1))
  (Default|UpdateInterface _returnvalue)
  (Development|PrintString "Strong")
  (Actor|DestroyActor))

(fn ConstructionScript)