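; Main menu Blueprint that lets the player start the game or quit through a MainMenu widget.
; On BeginPlay it casts the widget from its Widget component to MainMenu and binds click events to the Start and Exit buttons.
; Start opens the FirstLevel map by name, and Exit quits the game.
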(event Custom|OnClicked_Event_Start
  (Game|OpenLevel(byName) "FirstLevel"))

(event Custom|OnClicked_Event_Exit
  (Game|QuitGame 0 "Quit" false))

(event EventBeginPlay
  (bind _asmain_menu (Utilities|Casting|CastToMainMenu (UserInterface|GetWidget (Variables|Default|GetWidget))))
  (EventDispatchers|AssignOnClicked (Variables|/Game/Blueprints/MainMenu.MainMenu_C|GetStart_Button _asmain_menu) (delegate Custom|OnClicked_Event_Start))
  (EventDispatchers|AssignOnClicked (Variables|/Game/Blueprints/MainMenu.MainMenu_C|GetExit_Button _asmain_menu) (delegate Custom|OnClicked_Event_Exit)))

(fn ConstructionScript)