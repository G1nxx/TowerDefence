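; Tower build menu actor that lets the player buy a Basic, Splash or Sniper tower for a tower place.
; ShowWidget reveals the TowerWidget, binds its buttons and enables those affordable from MyMainBase money.
; A purchase deducts cost, spawns the tower and a PlaceToUpgrade, refreshes the base interface, hides the menu and destroys the tower place.
; PlaceToUpgrade receives the new tower, except for Splash, whose reference stays None.
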(event Custom|OnClicked_Event_SplashTower
  ;[0 0 0] Menu
  ;;[1 1 1] clickEvents
  ;;;[1 0 0] SplashTowerButtonClicked
  (if (>= (Variables|/Script/TowerDefence.MainBase|GetMoneyInGame (stale Custom|ShowWidget _returnvalue_2)) (Variables|/Script/TowerDefence.MainBase|GetSplashTowerCost (stale Custom|ShowWidget _returnvalue_2)))
    (Variables|/Script/TowerDefence.MainBase|SetMoneyInGame (stale Custom|ShowWidget _returnvalue_2) (- (Variables|/Script/TowerDefence.MainBase|GetMoneyInGame (stale Custom|ShowWidget _returnvalue_2)) (Variables|/Script/TowerDefence.MainBase|GetSplashTowerCost (stale Custom|ShowWidget _returnvalue_2))))
    (Game|SpawnActorfromClass "/Game/Blueprints/MySplashTower.MySplashTower_C" (Transformation|GetActorTransform (Variables|Default|GetTowerPlaceToInteract)) "Undefined" "MultiplyWithRoot" 0 0)
    (bind _returnvalue (Game|SpawnActorfromClass "/Game/Blueprints/PlaceToUpgrade.PlaceToUpgrade_C" (Transformation|GetActorTransform (Variables|Default|GetTowerPlaceToInteract)) "Undefined" "MultiplyWithRoot" 0 0))
    (Variables|/Game/Blueprints/PlaceToUpgrade.PlaceToUpgrade_C|SetTowerToInteract _returnvalue 0)
    (bind _returnvalue_2 (Actor|GetActorOfClass "/Game/Blueprints/MyMainBase.MyMainBase_C"))
    (Default|UpdateInterface _returnvalue_2)
    (Widget|SetVisibility (UserInterface|GetWidget (Variables|Default|GetWidget)) "Hidden")
    (Actor|DestroyActor (Variables|Default|GetTowerPlaceToInteract))))

(event Custom|OnClicked_Event_SniperTower
  ;[0 0 0] Menu
  ;;[1 1 1] clickEvents
  ;;;[0.0534 1 0] SniperTowerButtonClicked
  (if (>= (Variables|/Script/TowerDefence.MainBase|GetMoneyInGame (stale Custom|ShowWidget _returnvalue_2)) (Variables|/Script/TowerDefence.MainBase|GetSniperTowerCost (stale Custom|ShowWidget _returnvalue_2)))
    (Variables|/Script/TowerDefence.MainBase|SetMoneyInGame (stale Custom|ShowWidget _returnvalue_2) (- (Variables|/Script/TowerDefence.MainBase|GetMoneyInGame (stale Custom|ShowWidget _returnvalue_2)) (Variables|/Script/TowerDefence.MainBase|GetSniperTowerCost (stale Custom|ShowWidget _returnvalue_2))))
    (bind _returnvalue (Game|SpawnActorfromClass "/Game/Blueprints/MySniperTower.MySniperTower_C" (Transformation|GetActorTransform (Variables|Default|GetTowerPlaceToInteract)) "Undefined" "MultiplyWithRoot" 0 0))
    (bind _returnvalue_2 (Game|SpawnActorfromClass "/Game/Blueprints/PlaceToUpgrade.PlaceToUpgrade_C" (Transformation|GetActorTransform (Variables|Default|GetTowerPlaceToInteract)) "Undefined" "MultiplyWithRoot" 0 0))
    (Variables|/Game/Blueprints/PlaceToUpgrade.PlaceToUpgrade_C|SetTowerToInteract _returnvalue_2 _returnvalue)
    (bind _returnvalue_3 (Actor|GetActorOfClass "/Game/Blueprints/MyMainBase.MyMainBase_C"))
    (Default|UpdateInterface _returnvalue_3)
    (Widget|SetVisibility (UserInterface|GetWidget (Variables|Default|GetWidget)) "Hidden")
    (Actor|DestroyActor (Variables|Default|GetTowerPlaceToInteract))))

(event Custom|ShowWidget
  (bind _widget (Variables|Default|GetWidget))
  (bind _returnvalue (UserInterface|GetWidget _widget))
  ;[0 0 0] Menu
  ;;[1 1 1] OnCLicked
  (bind _astower_widget (Utilities|Casting|CastToTowerWidget _returnvalue)
    (:then
      (Widget|SetVisibility _returnvalue "Visible")
      (Development|PrintString "Clicked")
      (bind _returnvalue_2 (Actor|GetActorOfClass "/Game/Blueprints/MyMainBase.MyMainBase_C"))
      ;;[1 1 1] clickEvents
      ;;;[0 0.04559 1] BasicTowerButtonClicked
      (EventDispatchers|AssignOnClicked (Variables|/Game/Blueprints/TowerWidget.TowerWidget_C|GetBasicTowerButton _astower_widget) (delegate Custom|OnClicked_Event_BasicTower))
      (Widget|SetIsEnabled (Variables|/Game/Blueprints/TowerWidget.TowerWidget_C|GetBasicTowerButton _astower_widget) (>= (Variables|/Script/TowerDefence.MainBase|GetMoneyInGame _returnvalue_2) (Variables|/Script/TowerDefence.MainBase|GetBasicTowerCost _returnvalue_2)))
      ;;;[1 0 0] SplashTowerButtonClicked
      (EventDispatchers|AssignOnClicked (Variables|/Game/Blueprints/TowerWidget.TowerWidget_C|GetSplashTowerButton _astower_widget) (delegate Custom|OnClicked_Event_SplashTower))
      (Widget|SetIsEnabled (Variables|/Game/Blueprints/TowerWidget.TowerWidget_C|GetSplashTowerButton _astower_widget) (>= (Variables|/Script/TowerDefence.MainBase|GetMoneyInGame _returnvalue_2) (Variables|/Script/TowerDefence.MainBase|GetSplashTowerCost _returnvalue_2)))
      ;;;[0.0534 1 0] SniperTowerButtonClicked
      (EventDispatchers|AssignOnClicked (Variables|/Game/Blueprints/TowerWidget.TowerWidget_C|GetSniperTowerButton _astower_widget) (delegate Custom|OnClicked_Event_SniperTower))
      (Widget|SetIsEnabled (Variables|/Game/Blueprints/TowerWidget.TowerWidget_C|GetSniperTowerButton _astower_widget) (>= (Variables|/Script/TowerDefence.MainBase|GetMoneyInGame _returnvalue_2) (Variables|/Script/TowerDefence.MainBase|GetSniperTowerCost _returnvalue_2))))
    (:CastFailed
      (Development|PrintString "Fail to connect menu"))))

(event Custom|OnClicked_Event_BasicTower
  ;[0 0 0] Menu
  ;;[1 1 1] clickEvents
  ;;;[0 0.04559 1] BasicTowerButtonClicked
  (if (>= (Variables|/Script/TowerDefence.MainBase|GetMoneyInGame (stale Custom|ShowWidget _returnvalue_2)) (Variables|/Script/TowerDefence.MainBase|GetBasicTowerCost (stale Custom|ShowWidget _returnvalue_2)))
    (Variables|/Script/TowerDefence.MainBase|SetMoneyInGame (stale Custom|ShowWidget _returnvalue_2) (- (Variables|/Script/TowerDefence.MainBase|GetMoneyInGame (stale Custom|ShowWidget _returnvalue_2)) (Variables|/Script/TowerDefence.MainBase|GetBasicTowerCost (stale Custom|ShowWidget _returnvalue_2))))
    (bind _returnvalue (Game|SpawnActorfromClass "/Game/Blueprints/MyBasicTower.MyBasicTower_C" (Transformation|GetActorTransform (Variables|Default|GetTowerPlaceToInteract)) "Undefined" "MultiplyWithRoot" 0 0))
    (bind _returnvalue_2 (Game|SpawnActorfromClass "/Game/Blueprints/PlaceToUpgrade.PlaceToUpgrade_C" (Transformation|GetActorTransform (Variables|Default|GetTowerPlaceToInteract)) "Undefined" "MultiplyWithRoot" 0 0))
    (Variables|/Game/Blueprints/PlaceToUpgrade.PlaceToUpgrade_C|SetTowerToInteract _returnvalue_2 _returnvalue)
    (bind _returnvalue_3 (Actor|GetActorOfClass "/Game/Blueprints/MyMainBase.MyMainBase_C"))
    (Default|UpdateInterface _returnvalue_3)
    (Widget|SetVisibility (UserInterface|GetWidget (Variables|Default|GetWidget)) "Hidden")
    (Actor|DestroyActor (Variables|Default|GetTowerPlaceToInteract))))

(event EventBeginPlay
  ;[0 0 0] Menu
  ;;[1 1 1] HideAtStart
  (Widget|SetVisibility (UserInterface|GetWidget (Variables|Default|GetWidget)) "Hidden"))

(event Collision|EventActorBeginOverlap
  (params (OtherActor :type Actor%20Object%20Reference)))

(event EventTick
  (params (DeltaSeconds :type Float%20%28single-precision%29)))

(fn ConstructionScript)