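; Tower upgrade menu actor that lets the player upgrade or sell the tower in TowerToInteract through an UpgradeWidget, hidden at start.
; ShowWidget reveals it, hides the MenuForBuilding widget, caches MyMainBase and binds both buttons.
; Upgrade spends MoneyInGame to raise the level up to 10 and updates the labels.
; Destroy refunds part of the cost, swaps the tower for a PlaceToBuild, and, like Upgrade, refreshes the base interface.
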(event Custom|OnClicked_Event_Destroy
  (bind _towertointeract (Variables|Default|GetTowerToInteract))
  ;[0 0 0] Menu
  ;;[1 1 1] clickEvents
  ;;;[1 0 0] DestroyButtonClicked
  (bind _asabstract_tower (Utilities|Casting|CastToAbstractTower (Variables|Default|GetTowerToInteract)))
  (Variables|/Script/TowerDefence.MainBase|SetMoneyInGame (stale Custom|ShowWidget _returnvalue_3) (+ (Variables|/Script/TowerDefence.MainBase|GetMoneyInGame (stale Custom|ShowWidget _returnvalue_3)) (/ (Variables|/Script/TowerDefence.AbstractTower|GetCostOfTower _asabstract_tower) 2) (* (/ (* (- (Variables|/Script/TowerDefence.AbstractTower|GetLevelOfTower _asabstract_tower) 1) (/ (Variables|/Script/TowerDefence.AbstractTower|GetCostOfTower _asabstract_tower) 2)) 3) 2)))
  (Game|SpawnActorfromClass "/Game/Blueprints/PlaceToBuild.PlaceToBuild_C" (Math|Transform|MakeTransform (.location (Transformation|GetActorTransform _towertointeract)) "0, 0, 0" "1.000000,1.000000,1.000000") "Undefined" "MultiplyWithRoot" 0 0)
  (Actor|DestroyActor _towertointeract)
  (Actor|DestroyActor (Variables|Default|GetUpgradePlace))
  (Widget|SetVisibility (UserInterface|GetWidget (Variables|Default|GetWidget)) "Hidden")
  (bind _returnvalue (Actor|GetActorOfClass "/Game/Blueprints/MyMainBase.MyMainBase_C"))
  (Default|UpdateInterface _returnvalue))

(event Custom|OnClicked_Event_Upgrade
  ;[0 0 0] Menu
  ;;[1 1 1] clickEvents
  ;;;[0.0534 1 0] UpgradeButtonClicked
  (bind _asabstract_tower (Utilities|Casting|CastToAbstractTower (Variables|Default|GetTowerToInteract)))
  (if (< (Variables|/Script/TowerDefence.AbstractTower|GetLevelOfTower _asabstract_tower) 10)
    (if (>= (Variables|/Script/TowerDefence.MainBase|GetMoneyInGame (stale Custom|ShowWidget _returnvalue_3)) (Variables|/Script/TowerDefence.AbstractTower|GetCostOfUpgrading _asabstract_tower))
      (Widget|SetIsEnabled (Variables|/Game/Blueprints/UpgradeWidget.UpgradeWidget_C|GetUpgradeButton (stale Custom|ShowWidget _asupgrade_widget)) (>= (Variables|/Script/TowerDefence.MainBase|GetMoneyInGame (stale Custom|ShowWidget _returnvalue_3)) (Variables|/Script/TowerDefence.AbstractTower|GetCostOfUpgrading _asabstract_tower)))
      (Variables|/Script/TowerDefence.MainBase|SetMoneyInGame (stale Custom|ShowWidget _returnvalue_3) (- (Variables|/Script/TowerDefence.MainBase|GetMoneyInGame (stale Custom|ShowWidget _returnvalue_3)) (Variables|/Script/TowerDefence.AbstractTower|GetCostOfUpgrading _asabstract_tower)))
      (Class|AbstractTower|UpdateLevel _asabstract_tower)
      (Variables|/Script/UMG.TextBlock|SetText (Variables|/Game/Blueprints/UpgradeWidget.UpgradeWidget_C|GetTextBlock_Level (stale Custom|ShowWidget _asupgrade_widget)) (Utilities|Text|ToText(Integer) (Variables|/Script/TowerDefence.AbstractTower|GetLevelOfTower _asabstract_tower)))
      (if (== (Variables|/Script/TowerDefence.AbstractTower|GetLevelOfTower _asabstract_tower) 10)
        (Variables|/Script/UMG.TextBlock|SetText (Variables|/Game/Blueprints/UpgradeWidget.UpgradeWidget_C|GetTextBlock_Cost (stale Custom|ShowWidget _asupgrade_widget)) "Max level")
        (else
          (Variables|/Script/UMG.TextBlock|SetText (Variables|/Game/Blueprints/UpgradeWidget.UpgradeWidget_C|GetTextBlock_Cost (stale Custom|ShowWidget _asupgrade_widget)) (Utilities|Text|ToText(Integer) (Variables|/Script/TowerDefence.AbstractTower|GetCostOfUpgrading _asabstract_tower)))))
      (bind _returnvalue (Actor|GetActorOfClass "/Game/Blueprints/MyMainBase.MyMainBase_C"))
      (Default|UpdateInterface _returnvalue))))

(event Custom|ShowWidget
  (bind _widget (Variables|Default|GetWidget))
  (bind _returnvalue (UserInterface|GetWidget _widget))
  ;[0 0 0] Menu
  ;;[1 1 1] OnCLicked
  (bind _asupgrade_widget (Utilities|Casting|CastToUpgradeWidget _returnvalue)
    (:then
      (Widget|SetVisibility _returnvalue "Visible")
      (Development|PrintString "Clicked")
      (bind _returnvalue_2 (Actor|GetActorOfClass "/Game/Blueprints/MenuForBuilding.MenuForBuilding_C"))
      (bind _astower_widget (Utilities|Casting|CastToTowerWidget (UserInterface|GetWidget (Variables|/Game/Blueprints/MenuForBuilding.MenuForBuilding_C|GetWidget _returnvalue_2))))
      ;;[1 1 1] clickEvents
      (Widget|SetVisibility _astower_widget "Hidden")
      (bind _returnvalue_3 (Actor|GetActorOfClass "/Game/Blueprints/MyMainBase.MyMainBase_C"))
      ;;;[1 0 0] DestroyButtonClicked
      (EventDispatchers|BindEventtoOnClicked (Variables|/Game/Blueprints/UpgradeWidget.UpgradeWidget_C|GetDestroyButton _asupgrade_widget) (delegate Custom|OnClicked_Event_Destroy))
      ;;;[0.0534 1 0] UpgradeButtonClicked
      (EventDispatchers|AssignOnClicked (Variables|/Game/Blueprints/UpgradeWidget.UpgradeWidget_C|GetUpgradeButton _asupgrade_widget) (delegate Custom|OnClicked_Event_Upgrade))
      (Widget|SetIsEnabled (Variables|/Game/Blueprints/UpgradeWidget.UpgradeWidget_C|GetUpgradeButton _asupgrade_widget) true)
      (Development|PrintString "end"))
    (:CastFailed
      (Development|PrintString "Fail to connect menu"))))

(event EventBeginPlay
  ;[0 0 0] Menu
  ;;[1 1 1] HideAtStart
  (Widget|SetVisibility (UserInterface|GetWidget (Variables|Default|GetWidget)) "Hidden"))

(event Collision|EventActorBeginOverlap
  (params (OtherActor :type Actor%20Object%20Reference)))

(event EventTick
  (params (DeltaSeconds :type Float%20%28single-precision%29)))

(fn ConstructionScript)