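; Basic enemy actor for a tower defense game that damages the main base or pays a bounty when killed.
; EnemyatBase takes one health from MyMainBase, while EnemyIsKilled adds ValueForKilling to its money and prints the total; both refresh the base interface and destroy the enemy.
; A kill also re-enables or disables the TowerWidget purchase buttons on MenuForBuilding by comparing money to each tower cost.
; Other actors are found through GetActorOfClass lookups.
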(event EventEnemyIsKilled
  ;[1 1 1] EnemyIsKilled
  (bind _returnvalue (Actor|GetActorOfClass "/Game/Blueprints/MyMainBase.MyMainBase_C"))
  (bind _output_get (Variables|/Script/TowerDefence.MainBase|SetMoneyInGame _returnvalue (Math|Float|Truncate (+ (Variables|/Script/TowerDefence.MainBase|GetMoneyInGame _returnvalue) (Variables|Default|GetValueForKilling)))))
  (Default|UpdateInterface _returnvalue)
  (Development|PrintString (Utilities|String|ToString(Integer) _output_get) true true "(R=0.040479,G=1.000000,B=0.074658,A=1.000000)")
  (bind _returnvalue_2 (Actor|GetActorOfClass "/Game/Blueprints/MenuForBuilding.MenuForBuilding_C"))
  (bind _astower_widget (Utilities|Casting|CastToTowerWidget (UserInterface|GetWidget (Variables|/Game/Blueprints/MenuForBuilding.MenuForBuilding_C|GetWidget _returnvalue_2))))
  (bind _returnvalue_3 (Actor|GetActorOfClass "/Game/Blueprints/MyMainBase.MyMainBase_C"))
  (Widget|SetIsEnabled (Variables|/Game/Blueprints/TowerWidget.TowerWidget_C|GetBasicTowerButton _astower_widget) (> (Variables|/Script/TowerDefence.MainBase|GetMoneyInGame _returnvalue_3) (Variables|/Script/TowerDefence.MainBase|GetBasicTowerCost _returnvalue_3)))
  (Widget|SetIsEnabled (Variables|/Game/Blueprints/TowerWidget.TowerWidget_C|GetSplashTowerButton _astower_widget) (> (Variables|/Script/TowerDefence.MainBase|GetMoneyInGame _returnvalue_3) (Variables|/Script/TowerDefence.MainBase|GetSplashTowerCost _returnvalue_3)))
  (Widget|SetIsEnabled (Variables|/Game/Blueprints/TowerWidget.TowerWidget_C|GetSniperTowerButton _astower_widget) (> (Variables|/Script/TowerDefence.MainBase|GetMoneyInGame _returnvalue_3) (Variables|/Script/TowerDefence.MainBase|GetSniperTowerCost _returnvalue_3)))
  (Actor|DestroyActor))

(event EventBeginPlay
  (Variables|Default|SetValueForKilling 3))

(event EventEnemyatBase
  ;[1 1 1] EnemyAtBase
  (bind _returnvalue (Actor|GetActorOfClass "/Game/Blueprints/MyMainBase.MyMainBase_C"))
  (Variables|/Script/TowerDefence.MainBase|SetHealthOfMainBase _returnvalue (- (Variables|/Script/TowerDefence.MainBase|GetHealthOfMainBase _returnvalue) 1))
  (Default|UpdateInterface _returnvalue)
  (Actor|DestroyActor))

(fn ConstructionScript)

(fn OnRepMainBase)