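; Main base actor that holds the game's base health and money values and displays them in a UI widget.
; BeginPlay sets the starting health and money, then calls UpdateInterface.
; UpdateInterface casts the Intrface component's widget to Interface and writes both values into its text blocks, reading them through GetActorOfClass rather than self.
; Nothing in this file changes the values after initialization.
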(event Custom|UpdateInterface
  (bind _asinterface (Utilities|Casting|CastToInterface (UserInterface|GetWidget (Variables|Default|GetIntrface))))
  (bind _returnvalue (Actor|GetActorOfClass "MyMainBase_C"))
  (Variables|/Script/UMG.TextBlock|SetText (Variables|/Game/Blueprints/Interface.Interface_C|GetTextBlock_Health _asinterface) (Utilities|Text|ToText(Integer) (Variables|/Script/TowerDefence.MainBase|GetHealthOfMainBase _returnvalue)))
  (Variables|/Script/UMG.TextBlock|SetText (Variables|/Game/Blueprints/Interface.Interface_C|GetTextBlock_Money _asinterface) (Utilities|Text|ToText(Integer) (Variables|/Script/TowerDefence.MainBase|GetMoneyInGame _returnvalue))))

(event EventBeginPlay
  (Variables|Default|SetMoneyInGame 100)
  (Variables|Default|SetHealthOfMainBase 20)
  (CallFunction|UpdateInterface))

(event Collision|EventActorBeginOverlap
  (params (OtherActor :type Actor%20Object%20Reference)))

(event EventTick
  (params (DeltaSeconds :type Float%20%28single-precision%29)))

(fn ConstructionScript)