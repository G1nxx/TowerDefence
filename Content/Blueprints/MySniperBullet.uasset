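; Sniper bullet actor that damages enemies it overlaps.
; Its Sphere overlap checks for the "Enemy" tag, casts to AbstractEnemy and calls TakeDamage, with base Damage raised by a tenth per LevelOfDamage.
; After a hit it prints a debug string and destroys itself, while overlaps with other actors are ignored.
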(event OnComponentBeginOverlap(Sphere)
  (params (OverlappedComponent :type Primitive%20Component%20Object%20Reference) (OtherActor :type Actor%20Object%20Reference) (OtherComp :type Primitive%20Component%20Object%20Reference) (OtherBodyIndex :type Integer) (bFromSweep :type Boolean) (SweepResult :type Hit%20Result%20Structure%20%28by%20ref%29))
  (if (Actor|ActorHasTag OtherActor "Enemy")
    (bind _asabstract_enemy (Utilities|Casting|CastToAbstractEnemy OtherActor))
    (Class|AbstractEnemy|TakeDamage _asabstract_enemy (/ (* (Variables|Default|Getdamage) (+ (Variables|Default|GetlevelOfDamage) 10)) 10))
    (Development|PrintString "Hello" true true "(R=1.000000,G=0.567016,B=0.151122,A=1.000000)")
    (Actor|DestroyActor)))

(fn ConstructionScript)