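; MySplashBullet is a projectile Blueprint that deals area damage to basic enemies and destroys itself on impact.
; When its Sphere overlaps an actor tagged BasicEnemy, it loops over the actors overlapping DamageSphere and calls TakeDamage on each MyBasicEnemy.
; The damage amount scales linearly with LevelOfDamage.
; The loop stops at the first actor that fails the cast, so enemies later in the list take no damage.
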(event OnComponentBeginOverlap(Sphere)
  (params (OverlappedComponent :type Primitive%20Component%20Object%20Reference) (OtherActor :type Actor%20Object%20Reference) (OtherComp :type Primitive%20Component%20Object%20Reference) (OtherBodyIndex :type Integer) (bFromSweep :type Boolean) (SweepResult :type Hit%20Result%20Structure%20%28by%20ref%29))
  (if (Actor|ActorHasTag OtherActor "BasicEnemy")
    (bind _array_element (Utilities|Array|ForEachLoopwithBreak (Collision|GetOverlappingActors (Variables|Default|GetDamageSphere) 0 :!class /Script/Engine.PrimitiveComponent) :!label _label)
      (:LoopBody
        (bind _asmy_basic_enemy (Utilities|Casting|CastToMyBasicEnemy _array_element)
          (:then
            (Class|AbstractEnemy|TakeDamage _asmy_basic_enemy (/ (* (Variables|Default|Getdamage) (+ (* (Variables|Default|GetlevelOfDamage) 2) 10)) 10)))
          (:CastFailed
            (goto _label Break))))
      (:Completed
        (Actor|DestroyActor)))))

(fn ConstructionScript)