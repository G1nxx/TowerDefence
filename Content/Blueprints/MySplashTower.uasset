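; MySplashTower is a clickable tower that keeps track of enemies in range and connects to the upgrade menu.
; Clicking its MovingPart fills the MenuForUpgrading widget with cost and level, registers the tower and shows it; at level 10 it only sets "Max level" text.
; Sphere overlaps with "Enemy"-tagged actors rebuild AllEnemies from overlapping AbstractEnemy actors.
; This graph contains no firing logic.
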(event OnComponentBeginOverlap(Sphere)
  (params (OverlappedComponent :type Primitive%20Component%20Object%20Reference) (OtherActor :type Actor%20Object%20Reference) (OtherComp :type Primitive%20Component%20Object%20Reference) (OtherBodyIndex :type Integer) (bFromSweep :type Boolean) (SweepResult :type Hit%20Result%20Structure%20%28by%20ref%29))
  ;[1 1 1] ChoosingWhichToShoot
  (if (Actor|ActorHasTag OtherActor "Enemy")
    (Utilities|Array|Clear (Variables|Default|GetAllEnemies))
    (Variables|Default|SetAllEnemies (Collision|GetOverlappingActors (Variables|Default|GetSphere) "/Script/TowerDefence.AbstractEnemy" :!class /Script/Engine.PrimitiveComponent))))

(event OnClicked(MovingPart)
  (params (TouchedComponent :type Primitive%20Component%20Object%20Reference) (ButtonPressed :type Key%20Structure :default "None"))
  (bind _self self)
  (bind _leveloftower (Variables|/Script/TowerDefence.AbstractTower|GetLevelOfTower _self))
  (bind _returnvalue (Actor|GetActorOfClass "/Game/Blueprints/MenuForUpgrading.MenuForUpgrading_C"))
  (bind _asupgrade_widget (Utilities|Casting|CastToUpgradeWidget (UserInterface|GetWidget (Variables|/Game/Blueprints/MenuForUpgrading.MenuForUpgrading_C|GetWidget _returnvalue))))
  (if (== _leveloftower 10)
    (Variables|/Script/UMG.TextBlock|SetText (Variables|/Game/Blueprints/UpgradeWidget.UpgradeWidget_C|GetTextBlock_Cost _asupgrade_widget) "Max level")
    (else
      (Variables|/Script/UMG.TextBlock|SetText (Variables|/Game/Blueprints/UpgradeWidget.UpgradeWidget_C|GetTextBlock_Cost _asupgrade_widget) (Utilities|Text|ToText(Integer) (Variables|/Script/TowerDefence.AbstractTower|GetCostOfUpgrading _self)))
      (Variables|/Script/UMG.TextBlock|SetText (Variables|/Game/Blueprints/UpgradeWidget.UpgradeWidget_C|GetTextBlock_Level _asupgrade_widget) (Utilities|Text|ToText(Integer) _leveloftower))
      (Variables|/Game/Blueprints/MenuForUpgrading.MenuForUpgrading_C|SetTowerToInteract _returnvalue self)
      (Variables|/Game/Blueprints/MenuForUpgrading.MenuForUpgrading_C|SetUpgradePlace _returnvalue 0)
      (Default|ShowWidget _returnvalue))))

(event OnComponentEndOverlap(Sphere)
  (params (OverlappedComponent :type Primitive%20Component%20Object%20Reference) (OtherActor :type Actor%20Object%20Reference) (OtherComp :type Primitive%20Component%20Object%20Reference) (OtherBodyIndex :type Integer))
  ;[1 1 1] ChoosingWhichToShoot
  (if (Actor|ActorHasTag OtherActor "Enemy")
    (Variables|Default|SetAllEnemies (Collision|GetOverlappingActors (Variables|Default|GetSphere) "/Script/TowerDefence.AbstractEnemy" :!class /Script/Engine.PrimitiveComponent))))

(event EventClickedonTower
  (bind _self self)
  (bind _leveloftower (Variables|/Script/TowerDefence.AbstractTower|GetLevelOfTower _self))
  (bind _returnvalue (Actor|GetActorOfClass "/Game/Blueprints/MenuForUpgrading.MenuForUpgrading_C"))
  (bind _asupgrade_widget (Utilities|Casting|CastToUpgradeWidget (UserInterface|GetWidget (Variables|/Game/Blueprints/MenuForUpgrading.MenuForUpgrading_C|GetWidget _returnvalue))))
  (if (== _leveloftower 10)
    (Variables|/Script/UMG.TextBlock|SetText (Variables|/Game/Blueprints/UpgradeWidget.UpgradeWidget_C|GetTextBlock_Cost _asupgrade_widget) "Max level")
    (else
      (Variables|/Script/UMG.TextBlock|SetText (Variables|/Game/Blueprints/UpgradeWidget.UpgradeWidget_C|GetTextBlock_Cost _asupgrade_widget) (Utilities|Text|ToText(Integer) (Variables|/Script/TowerDefence.AbstractTower|GetCostOfUpgrading _self)))
      (Variables|/Script/UMG.TextBlock|SetText (Variables|/Game/Blueprints/UpgradeWidget.UpgradeWidget_C|GetTextBlock_Level _asupgrade_widget) (Utilities|Text|ToText(Integer) _leveloftower))
      (Variables|/Game/Blueprints/MenuForUpgrading.MenuForUpgrading_C|SetTowerToInteract _returnvalue self)
      (Variables|/Game/Blueprints/MenuForUpgrading.MenuForUpgrading_C|SetUpgradePlace _returnvalue 0)
      (Default|ShowWidget _returnvalue))))

(fn ConstructionScript)