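; PlaceToUpgrade is a clickable sprite spot that opens the upgrade menu for its associated tower.
; On click, it finds the MenuForUpgrading actor and writes the tower's current level into that actor's UpgradeWidget.
; It then hands the menu both the tower and itself before showing the widget.
; The click handler also prints a leftover-looking debug string, and the construction script is empty.
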(event OnClicked(PaperSprite)
  (params (TouchedComponent :type Primitive%20Component%20Object%20Reference) (ButtonPressed :type Key%20Structure :default "None"))
  (Development|PrintString "Hello")
  (bind _returnvalue (Actor|GetActorOfClass "/Game/Blueprints/MenuForUpgrading.MenuForUpgrading_C"))
  (bind _asabstract_tower (Utilities|Casting|CastToAbstractTower (Variables|Default|GetTowerToInteract)))
  (bind _asupgrade_widget (Utilities|Casting|CastToUpgradeWidget (UserInterface|GetWidget (Variables|/Game/Blueprints/MenuForUpgrading.MenuForUpgrading_C|GetWidget _returnvalue))))
  (Variables|/Script/UMG.TextBlock|SetText (Variables|/Game/Blueprints/UpgradeWidget.UpgradeWidget_C|GetTextBlock_Level _asupgrade_widget) (Utilities|Text|ToText(Integer) (Variables|/Script/TowerDefence.AbstractTower|GetLevelOfTower _asabstract_tower)))
  (Variables|/Game/Blueprints/MenuForUpgrading.MenuForUpgrading_C|SetTowerToInteract _returnvalue (Variables|Default|GetTowerToInteract))
  (Variables|/Game/Blueprints/MenuForUpgrading.MenuForUpgrading_C|SetUpgradePlace _returnvalue self)
  (Default|ShowWidget _returnvalue))

(fn ConstructionScript)