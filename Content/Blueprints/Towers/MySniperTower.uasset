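; Sniper tower Blueprint that chooses which enemies to target and opens an upgrade menu when clicked.
; Clicks fill the upgrade widget with cost and level, then hand the tower and its placement to the menu actor; at level ten, only "Max level" text is set.
; Sphere overlap changes rebuild AllEnemies, keeping only StrongEnemy actors when any are in range, otherwise all AbstractEnemy actors.
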(event OnComponentBeginOverlap(Sphere)
  (params (OverlappedComponent :type Primitive%20Component%20Object%20Reference) (OtherActor :type Actor%20Object%20Reference) (OtherComp :type Primitive%20Component%20Object%20Reference) (OtherBodyIndex :type Integer) (bFromSweep :type Boolean) (SweepResult :type Hit%20Result%20Structure%20%28by%20ref%29))
  (bind _sphere (Variables|Default|GetSphere))
  (bind _overlappingactors (Collision|GetOverlappingActors _sphere "/Script/TowerDefence.StrongEnemy" :!class /Script/Engine.PrimitiveComponent))
  ;[1 1 1] ChoosingWhichToShoot
  (if (Actor|ActorHasTag OtherActor "Enemy")
    (Utilities|Array|Clear (Variables|Default|GetAllEnemies))
    (if (> (Utilities|Array|Length _overlappingactors) 0)
      (Variables|Default|SetAllEnemies _overlappingactors)
      (else
        (Variables|Default|SetAllEnemies (Collision|GetOverlappingActors (Variables|Default|GetSphere) "/Script/TowerDefence.AbstractEnemy" :!class /Script/Engine.PrimitiveComponent))))))

(event OnClicked(MovingPart)
  (params (TouchedComponent :type Primitive%20Component%20Object%20Reference) (ButtonPressed :type Key%20Structure))
  (bind _self self)
  (bind _leveloftower (Variables|/Script/TowerDefence.AbstractTower|GetLevelOfTower _self))
  (bind _returnvalue (Actor|GetActorOfClass "/Game/Blueprints/UI/MenuForUpgrading.MenuForUpgrading_C"))
  (bind _asupgrade_widget (Utilities|Casting|CastToUpgradeWidget (UserInterface|GetWidget (Variables|/Game/Blueprints/UI/MenuForUpgrading.MenuForUpgrading_C|GetWidget _returnvalue))))
  (if (== _leveloftower 10)
    (Variables|/Script/UMG.TextBlock|SetText (Variables|/Game/Blueprints/UI/Widgets/UpgradeWidget.UpgradeWidget_C|GetTextBlock_Cost _asupgrade_widget) "Max level")
    (else
      (Variables|/Script/UMG.TextBlock|SetText (Variables|/Game/Blueprints/UI/Widgets/UpgradeWidget.UpgradeWidget_C|GetTextBlock_Cost _asupgrade_widget) (Utilities|Text|ToText(Integer) (Variables|/Script/TowerDefence.AbstractTower|GetCostOfUpgrading _self)))
      (Variables|/Script/UMG.TextBlock|SetText (Variables|/Game/Blueprints/UI/Widgets/UpgradeWidget.UpgradeWidget_C|GetTextBlock_Level _asupgrade_widget) (Utilities|Text|ToText(Integer) _leveloftower))
      (Variables|/Game/Blueprints/UI/MenuForUpgrading.MenuForUpgrading_C|SetTowerToInteract _returnvalue self)
      (Variables|/Game/Blueprints/UI/MenuForUpgrading.MenuForUpgrading_C|SetUpgradePlace _returnvalue (Variables|Default|GetUpgradePlace))
      (Default|ShowWidget _returnvalue))))

(event OnComponentEndOverlap(Sphere)
  (params (OverlappedComponent :type Primitive%20Component%20Object%20Reference) (OtherActor :type Actor%20Object%20Reference) (OtherComp :type Primitive%20Component%20Object%20Reference) (OtherBodyIndex :type Integer))
  (bind _sphere (Variables|Default|GetSphere))
  (bind _overlappingactors (Collision|GetOverlappingActors _sphere "/Script/TowerDefence.StrongEnemy" :!class /Script/Engine.PrimitiveComponent))
  ;[1 1 1] ChoosingWhichToShoot
  (if (Actor|ActorHasTag OtherActor "Enemy")
    (if (> (Utilities|Array|Length _overlappingactors) 0)
      (Variables|Default|SetAllEnemies _overlappingactors)
      (else
        (Variables|Default|SetAllEnemies (Collision|GetOverlappingActors (Variables|Default|GetSphere) "/Script/TowerDefence.AbstractEnemy" :!class /Script/Engine.PrimitiveComponent))))))

(event EventClickedonTower
  (bind _self self)
  (bind _leveloftower (Variables|/Script/TowerDefence.AbstractTower|GetLevelOfTower _self))
  (bind _returnvalue (Actor|GetActorOfClass "/Game/Blueprints/UI/MenuForUpgrading.MenuForUpgrading_C"))
  (bind _asupgrade_widget (Utilities|Casting|CastToUpgradeWidget (UserInterface|GetWidget (Variables|/Game/Blueprints/UI/MenuForUpgrading.MenuForUpgrading_C|GetWidget _returnvalue))))
  (if (== _leveloftower 10)
    (Variables|/Script/UMG.TextBlock|SetText (Variables|/Game/Blueprints/UI/Widgets/UpgradeWidget.UpgradeWidget_C|GetTextBlock_Cost _asupgrade_widget) "Max level")
    (else
      (Variables|/Script/UMG.TextBlock|SetText (Variables|/Game/Blueprints/UI/Widgets/UpgradeWidget.UpgradeWidget_C|GetTextBlock_Cost _asupgrade_widget) (Utilities|Text|ToText(Integer) (Variables|/Script/TowerDefence.AbstractTower|GetCostOfUpgrading _self)))
      (Variables|/Script/UMG.TextBlock|SetText (Variables|/Game/Blueprints/UI/Widgets/UpgradeWidget.UpgradeWidget_C|GetTextBlock_Level _asupgrade_widget) (Utilities|Text|ToText(Integer) _leveloftower))
      (Variables|/Game/Blueprints/UI/MenuForUpgrading.MenuForUpgrading_C|SetTowerToInteract _returnvalue self)
      (Variables|/Game/Blueprints/UI/MenuForUpgrading.MenuForUpgrading_C|SetUpgradePlace _returnvalue (Variables|Default|GetUpgradePlace))
      (Default|ShowWidget _returnvalue))))

(fn ConstructionScript)